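; BP_Player is the player character Blueprint, which creates and shows WBP_HUD on the player's screen at BeginPlay.
; Jump debug helpers print apex time, air time, initial velocity and distance, but nothing in these graphs calls them, and the jump, land and Tick events are empty.
; A Hold macro uses a retriggerable delay and two gates to tell a tap from a held press.
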(event EventOnJumped)

(event EventOnLanded
  (params (Hit :type Hit%20Result%20Structure%20%28by%20ref%29)))

(event EventTick
  (params (DeltaSeconds :type Float%20%28single-precision%29)))

(event EventBeginPlay
  (CallFunction|CreateHUD))

(fn ConstructionScript)

(fn PrintApexTime
  (if (and (> (.z (Variables|Default|GetLastVelocity)) 0.0) (< (.z (Transformation|GetVelocity)) 0.0))
    (Development|PrintString "ApexTime:" true true "(R=1.000000,G=0.938499,B=0.000000,A=1.000000)" 1e+01)
    (Development|PrintString (Utilities|String|ToString(Float) (- (Utilities|Time|GetTimeSeconds) (Variables|Default|GetjumpStartTime))) true true "(R=1.000000,G=0.942341,B=0.000000,A=1.000000)" 1e+01))
  (Variables|Default|SetLastVelocity (Transformation|GetVelocity)))

(fn PrintJumpTime
  (Development|PrintString "JumpTime:" true true "(R=0.000000,G=0.660000,B=1.000000,A=1.000000)" 1e+01)
  (Development|PrintString (Utilities|String|ToString(Float) (- (Utilities|Time|GetTimeSeconds) (Variables|Default|GetjumpStartTime))) true true "(R=0.000000,G=0.660000,B=1.000000,A=1.000000)" 1e+01))

(fn PrintInitialVelocity
  (Variables|Default|SetStartPosition (Transformation|GetActorLocation))
  (Development|PrintString (Utilities|String|ToString(Vector) (Transformation|GetVelocity))))

(fn PrintJumpDistance
  (Development|PrintString "Jump distance:" true true "(R=0.000000,G=0.660000,B=1.000000,A=1.000000)" 5.0)
  (Development|PrintString (Utilities|String|ToString(Float) (Math|Vector|VectorLength (- (Transformation|GetActorLocation) (Variables|Default|GetStartPosition))))))

(fn CreateHUD
  (bind _returnvalue (UserInterface|CreateWidget "/Game/Tantrumn/Blueprints/UI/WBP_HUD.WBP_HUD_C"))
  (UserInterface|Viewport|AddtoPlayerScreen _returnvalue))